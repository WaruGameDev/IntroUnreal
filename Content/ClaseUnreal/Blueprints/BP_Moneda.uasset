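; BP_Moneda is an inventory pickup actor whose item is defined by an ItemData data table row handle.
; The construction script sets the static mesh from the matching row's Mesh.
; TocarSilla adds the row name and ValorSilla to the BPInventoryComponent on BP_GameModeExample, then destroys the actor.
; Nothing in this graph calls TocarSilla, and the overlap event is unused.
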(event `/Game/ClaseUnreal/Blueprints/Player/BPI_Interaccion.TocarSilla`
  (bind (_itemdata_datatable _itemdata_rowname) (break `DataTableRowHandle` (`self.ItemData`)))
  (`/Game/ClaseUnreal/Blueprints/BP_InventoryComponent.AgregarObjInventario` (`/Game/ClaseUnreal/Blueprints/Player/BP_GameModeExample.BP_InventoryComponent` (cast `/Game/ClaseUnreal/Blueprints/Player/BP_GameModeExample` (`GameplayStatics.GetGameMode`) :!pure true)) _itemdata_rowname (`self.ValorSilla`))
  (`self.K2_DestroyActor`))

(fn `UserConstructionScript`
  (bind (_itemdata_datatable _itemdata_rowname) (break `DataTableRowHandle` (`self.ItemData`)))
  (bind _returnvalue (`|GetDataTableRow` _itemdata_datatable _itemdata_rowname)
    (:`then`
      (`StaticMeshComponent.SetStaticMesh` (`self.StaticMesh`) (`.Mesh_14_3D1BC123493681CEBAE902A487761257` (break `/Game/ClaseUnreal/Data/S_InventoryItem` _returnvalue))))))