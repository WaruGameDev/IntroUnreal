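; Player controller Blueprint that toggles an inventory screen with the I key.
; When opened, it creates a new BPW_Inventory widget, adds it to the viewport, hides the item description and refreshes the contents.
; When closed, it removes that widget from its parent.
; An InventoryOpen flag tracks the state, and the mouse cursor is shown only while the inventory is open.
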(event `Key|I`
  (params (Key :type "Key Structure"))
  (:`Pressed`
    (if (`self.InventoryOpen`)
      (`Widget.RemoveFromParent` (`self.Inventory`))
      (set `self.InventoryOpen` false)
      (set `self.bShowMouseCursor` false)
      (else
        (bind _returnvalue (`|CreateWidget` "/Game/ClaseUnreal/Data/BPW_Inventory.BPW_Inventory_C"))
        (set `self.Inventory` _returnvalue)
        (`UserWidget.AddToViewport` _returnvalue 0)
        (`/Game/ClaseUnreal/Data/BPW_Inventory.HiddenDescItem` _returnvalue)
        (`/Game/ClaseUnreal/Data/BPW_Inventory.RefreshInvetory` _returnvalue)
        (set `self.InventoryOpen` true)
        (set `self.bShowMouseCursor` true)))))

(fn `UserConstructionScript`)